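; BP_Warlock is an overworld enemy that wanders at random.
; Its first Tick sets IsMoving and starts a looping BeginMoving event, which waits briefly, then either waits again or uses AIMoveTo toward a random reachable point around its current location.
; Only a successful move resumes the loop, and IsMoving is never cleared, so a failed move stops the wandering.
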(event Custom|BeginMoving
  (Utilities|FlowControl|Delay 2.0 :!label _label)
  (if (== (Math|Random|RandomIntegerinRange 0 1) 0)
    (AI|AIMoveTo self (.RandomLocation (AI|Navigation|GetRandomReachablePointinRadius (Transformation|GetActorLocation) 2e+03 0 0)) 0 5.0 false
      (:OnSuccess
        (goto _label)))
    (else
      (goto _label))))

(event Collision|EventActorBeginOverlap
  (params (OtherActor :type Actor%20Object%20Reference)))

(event EventTick
  (params (DeltaSeconds :type Float%20%28single-precision%29))
  (if (not (Variables|Default|GetIsMoving))
    (Variables|Default|SetIsMoving true)
    (CallFunction|BeginMoving)))

(fn ConstructionScript)