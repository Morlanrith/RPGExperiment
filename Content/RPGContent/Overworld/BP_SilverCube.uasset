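; BP_SilverCube is an RPG overworld pawn that wanders randomly and carries a randomized party of enemies.
; The construction script fills Enemies from EnemiesDataTable stats, always adding the first ValidEnemies row plus up to two random picks.
; BeginPlay and a one-time Tick check both start AI moves to reachable points nearby.
; After each successful move it pauses, with a coin flip deciding whether to move again or keep waiting.
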(event Custom|BeginMoving
  (AI|AIMoveTo self (.RandomLocation (AI|Navigation|GetRandomReachablePointinRadius (Transformation|GetActorLocation) 2e+03 0 0)) 0 5.0 false :!label _label
    (:OnSuccess
      (Utilities|FlowControl|Delay 2.0 :!label _label_2)
      (if (== (Math|Random|RandomIntegerinRange 0 1) 0)
        (goto _label)
        (else
          (goto _label_2))))))

(event Collision|EventActorBeginOverlap
  (params (OtherActor :type Actor%20Object%20Reference)))

(event EventTick
  (params (DeltaSeconds :type Float%20%28single-precision%29))
  (if (not (Variables|Default|GetMoving))
    (Variables|Default|SetMoving true)
    (CallFunction|BeginMoving)))

(event EventBeginPlay
  (CallFunction|BeginMoving))

(fn ConstructionScript
  (bind _validenemies (Variables|Default|GetValidEnemies))
  (bind _returnvalue (AddComponent|AddAdditionalOperations))
  (Variables|Default|SetEnemies _returnvalue)
  (CallFunction|AddEnemy (Utilities|Array|Get(acopy) _validenemies))
  (for _index (range 1 (Math|Random|RandomIntegerinRange 0 2))
    (CallFunction|AddEnemy (Utilities|Array|Get(acopy) _validenemies (Math|Random|RandomIntegerinRange 0 (- (Utilities|Array|Length _validenemies) 1))))))

(fn AddEnemy
  (params (Row :type Name :default "0"))
  (bind _returnvalue (Utilities|GetDataTableRow "/Game/RPGContent/DataTables/EnemiesDataTable.EnemiesDataTable" Row)
    (:then
      (Class|AdditionalOperations|AddPartyMemberStruct (Variables|Default|GetEnemies) (.Stats (Utilities|Struct|BreakEnemiesDataStructure _returnvalue))))))