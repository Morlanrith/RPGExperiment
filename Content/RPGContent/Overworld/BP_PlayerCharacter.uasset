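; Overworld player character with walk, look, jump and sprint controls that starts battles on touching a roaming enemy.
; Mesh overlap saves both parties, the player and enemy transforms, and the enemy's index (matched by transform) to BP_BattleInstance, then opens the combat level.
; BeginPlay restores position and party from that game instance.
; Tick restores game input and movement when no current enemy exists and movement is inactive.
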(event OnComponentBeginOverlap(Mesh)
  (params (OverlappedComponent :type Primitive%20Component%20Object%20Reference) (OtherActor :type Actor%20Object%20Reference) (OtherComp :type Primitive%20Component%20Object%20Reference) (OtherBodyIndex :type Integer) (bFromSweep :type Boolean) (SweepResult :type Hit%20Result%20Structure%20%28by%20ref%29))
  ;[1 1 1] Start Battle Elements
  (Variables|Default|GetCurrentEnemy
    (:then)
    (:else
      (bind _asroaming_enemy (Utilities|Casting|CastToRoamingEnemy OtherActor))
      (bind _asbp_battle_instance (Utilities|Casting|CastToBP_BattleInstance (Game|GetGameInstance)))
      (bind _returnvalue (Class|AdditionalOperations|GetParty (Variables|Default|GetPlayers)))
      (Variables|/Game/RPGContent/GameInstances/BP_BattleInstance.BP_BattleInstance_C|SetCurrentParty _asbp_battle_instance _returnvalue)
      (bind _returnvalue_2 (Class|AdditionalOperations|GetParty (Variables|/Script/RPGExperiment.RoamingEnemy|GetEnemies _asroaming_enemy)))
      (Variables|/Game/RPGContent/GameInstances/BP_BattleInstance.BP_BattleInstance_C|SetEncounteredEnemy _asbp_battle_instance _returnvalue_2)
      (Variables|/Game/RPGContent/GameInstances/BP_BattleInstance.BP_BattleInstance_C|SetPlayerPosition _asbp_battle_instance (Transformation|GetActorTransform))
      (for (_array_element _array_index) (Variables|/Game/RPGContent/GameInstances/BP_BattleInstance.BP_BattleInstance_C|GetRoamingEnemies _asbp_battle_instance)
        (Utilities|Array|Add (Variables|/Game/RPGContent/GameInstances/BP_BattleInstance.BP_BattleInstance_C|GetEnemyPositions _asbp_battle_instance) (Transformation|GetActorTransform _array_element))
        (if (== (Transformation|GetActorTransform _array_element) (Transformation|GetActorTransform _asroaming_enemy))
          (Variables|/Game/RPGContent/GameInstances/BP_BattleInstance.BP_BattleInstance_C|SetEnemyIndex _asbp_battle_instance _array_index)))
      (Game|OpenLevel(byName) "BasicCombatLevel1"))))

(event EventBeginPlay
  ;[1 1 1] Player Created
  (CallFunction|Spawnin))

(event EventTick
  (params (DeltaSeconds :type Float%20%28single-precision%29))
  (bind _playercontrol (Variables|Default|GetPlayerControl))
  ;[1 1 1] End Battle Elements
  (if (Math|Boolean|NORBoolean (Utilities|IsValid (Variables|Default|GetCurrentEnemy)) (Components|Activation|IsActive (Variables|Character|GetCharacterMovement)))
    (Input|SetInputModeGameOnly _playercontrol)
    (Variables|/Script/Engine.PlayerController|SetbShowMouseCursor _playercontrol false)
    (Components|Activation|Activate (Variables|Character|GetCharacterMovement) false)))

(event Input|ActionEvents|InputActionJump
  (params (Key :type Key%20Structure :default "None"))
  ;[1 1 1] Other Action Elements
  (:Pressed
    (Character|Jump))
  (:Released
    (Character|StopJumping)))

(event Input|ActionEvents|InputActionSprint
  (params (Key :type Key%20Structure :default "None"))
  (bind _charactermovement (Variables|Character|GetCharacterMovement))
  ;[1 1 1] Other Action Elements
  (:Pressed
    (Variables|/Script/Engine.CharacterMovementComponent|SetMaxWalkSpeed _charactermovement 1e+03))
  (:Released
    (Variables|/Script/Engine.CharacterMovementComponent|SetMaxWalkSpeed _charactermovement 6e+02)))

(event Input|AxisEvents|InputAxisMoveForward
  (params (AxisValue :type Float%20%28single-precision%29))
  ;[1 1 1] Movement Elements
  (Pawn|Input|AddMovementInput (Math|Vector|GetForwardVector (Math|Rotator|MakeRotator 0.0 0.0 (.Yaw (Math|Rotator|BreakRotator (Pawn|GetControlRotation :!class /Script/Engine.Pawn))))) AxisValue false))

(event Input|AxisEvents|InputAxisMoveRight
  (params (AxisValue :type Float%20%28single-precision%29))
  ;[1 1 1] Movement Elements
  (Pawn|Input|AddMovementInput (Math|Vector|GetRightVector (Math|Rotator|MakeRotator 0.0 0.0 (.Yaw (Math|Rotator|BreakRotator (Pawn|GetControlRotation :!class /Script/Engine.Pawn))))) AxisValue false))

(event Input|AxisEvents|InputAxisLookUp
  (params (AxisValue :type Float%20%28single-precision%29))
  ;[1 1 1] Rotation Elements
  (Pawn|Input|AddControllerPitchInput AxisValue))

(event Input|AxisEvents|InputAxisTurn
  (params (AxisValue :type Float%20%28single-precision%29))
  ;[1 1 1] Rotation Elements
  (Pawn|Input|AddControllerYawInput AxisValue))

(fn ConstructionScript)

(fn Spawnin
  (bind _output_get (Variables|Default|SetPlayerControl (Game|GetPlayerController 0)))
  (Input|SetInputModeGameOnly _output_get)
  (bind _asbp_battle_instance (Utilities|Casting|CastToBP_BattleInstance (Game|GetGameInstance)))
  (Transformation|SetActorTransform (Variables|/Game/RPGContent/GameInstances/BP_BattleInstance.BP_BattleInstance_C|GetPlayerPosition _asbp_battle_instance) false true)
  (Pawn|SetControlRotation _output_get (.Rotation (Math|Transform|BreakTransform (Variables|/Game/RPGContent/GameInstances/BP_BattleInstance.BP_BattleInstance_C|GetPlayerPosition _asbp_battle_instance))))
  (bind _asparty_player_state (Utilities|Casting|CastToPartyPlayerState (Variables|GetPlayerState)))
  (Class|AdditionalOperations|SetParty (Variables|/Script/RPGExperiment.PartyPlayerState|GetPlayerParty _asparty_player_state) (Variables|/Game/RPGContent/GameInstances/BP_BattleInstance.BP_BattleInstance_C|GetCurrentParty _asbp_battle_instance))
  (Variables|Default|SetPlayers (Variables|/Script/RPGExperiment.PartyPlayerState|GetPlayerParty _asparty_player_state)))