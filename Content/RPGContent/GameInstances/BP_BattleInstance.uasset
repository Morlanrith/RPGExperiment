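; BP_BattleInstance, in the GameInstances folder, holds RPG state for the party, player position and enemy encounters.
; LoadSaveValues casts a save object to MyPartySaveGame and copies its saved party and player position into the instance.
; ResetValues clears the encountered enemy, roaming enemy, enemy position and roaming ID collections, then zeroes the enemy index.
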(fn LoadSaveValues
  (params (SavedGame :type Save%20Game%20Object%20Reference))
  (bind _asmy_party_save_game (Utilities|Casting|CastToMyPartySaveGame SavedGame))
  (Variables|Default|SetCurrentParty (Variables|/Script/RPGExperiment.MyPartySaveGame|GetSavedParty _asmy_party_save_game))
  (Variables|Default|SetPlayerPosition (Variables|/Script/RPGExperiment.MyPartySaveGame|GetPlayerPos _asmy_party_save_game)))

(fn ResetValues
  (Utilities|Array|Clear (Variables|Default|GetEncounteredEnemy))
  (Utilities|Array|Clear (Variables|Default|GetRoamingEnemies))
  (Utilities|Array|Clear (Variables|Default|GetEnemyPositions))
  (Utilities|Array|Clear (Variables|Default|GetRoamingEnemyIDs))
  (Variables|Default|SetEnemyIndex 0))